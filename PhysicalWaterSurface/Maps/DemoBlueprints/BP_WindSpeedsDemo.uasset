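; Demo driver for the physical water surface that shows wind speed and fetch length presets across thirteen scale steps.
; BeginPlay goes fullscreen, adds the SceneInfo HUD and saves the initial camera transform.
; Tick reads Scale from NewGameInstance, applies that step's preset through WaterSettings.ConstructionEvent, updates the HUD and offsets the camera for steps above zero.
; Each branch ends in a SceneDelay-based Delay with nothing after it; Scale never changes here.
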(event EventBeginPlay
  (Utilities|FlowControl|Sequence
    (:then_0
      ;[1 1 1] console commands
      (Development|ExecuteConsoleCommand "fullscreen"))
    (:then_1
      ;[1 1 1] HUD
      (bind _returnvalue (UserInterface|CreateWidget "/Game/PhysicalWaterSurface/Blueprints/UI/SceneInfo.SceneInfo_C"))
      (bind _output_get (Variables|Default|SetHUD%20Reference _returnvalue))
      (UserInterface|Viewport|AddtoViewport _output_get 0))
    (:then_2
      ;[1 1 1] save initial camera transform
      (Variables|Default|SetInitialCameraTransform (Transformation|GetActorTransform (Variables|Default|GetCaneraActor))))))

(event EventActorBeginOverlap
  (params (OtherActor :type Actor%20Object%20Reference)))

(event EventTick
  (params (DeltaSeconds :type Float%20%28single-precision%29))
  (bind _watersettings (Variables|Default|GetWaterSettings))
  (bind _watersettings_2 (Variables|Default|GetWaterSettings))
  (bind _watersettings_3 (Variables|Default|GetWaterSettings))
  (bind _watersettings_4 (Variables|Default|GetWaterSettings))
  (bind _watersettings_5 (Variables|Default|GetWaterSettings))
  (bind _watersettings_6 (Variables|Default|GetWaterSettings))
  (bind _watersettings_7 (Variables|Default|GetWaterSettings))
  (bind _watersettings_8 (Variables|Default|GetWaterSettings))
  (bind _hud_reference (Variables|Default|GetHUD%20Reference))
  (bind _hud_reference_2 (Variables|Default|GetHUD%20Reference))
  (bind _initialcameratransform (Variables|Default|GetInitialCameraTransform))
  (bind _hud_reference_3 (Variables|Default|GetHUD%20Reference))
  (bind _initialcameratransform_2 (Variables|Default|GetInitialCameraTransform))
  (bind _hud_reference_4 (Variables|Default|GetHUD%20Reference))
  (bind _initialcameratransform_3 (Variables|Default|GetInitialCameraTransform))
  (bind _hud_reference_5 (Variables|Default|GetHUD%20Reference))
  (bind _initialcameratransform_4 (Variables|Default|GetInitialCameraTransform))
  (bind _hud_reference_6 (Variables|Default|GetHUD%20Reference))
  (bind _initialcameratransform_5 (Variables|Default|GetInitialCameraTransform))
  (bind _hud_reference_7 (Variables|Default|GetHUD%20Reference))
  (bind _initialcameratransform_6 (Variables|Default|GetInitialCameraTransform))
  (bind _hud_reference_8 (Variables|Default|GetHUD%20Reference))
  (bind _initialcameratransform_7 (Variables|Default|GetInitialCameraTransform))
  (bind _watersettings_9 (Variables|Default|GetWaterSettings))
  (bind _hud_reference_9 (Variables|Default|GetHUD%20Reference))
  (bind _initialcameratransform_8 (Variables|Default|GetInitialCameraTransform))
  (bind _watersettings_10 (Variables|Default|GetWaterSettings))
  (bind _hud_reference_10 (Variables|Default|GetHUD%20Reference))
  (bind _initialcameratransform_9 (Variables|Default|GetInitialCameraTransform))
  (bind _watersettings_11 (Variables|Default|GetWaterSettings))
  (bind _hud_reference_11 (Variables|Default|GetHUD%20Reference))
  (bind _initialcameratransform_10 (Variables|Default|GetInitialCameraTransform))
  (bind _watersettings_12 (Variables|Default|GetWaterSettings))
  (bind _hud_reference_12 (Variables|Default|GetHUD%20Reference))
  (bind _initialcameratransform_11 (Variables|Default|GetInitialCameraTransform))
  (bind _watersettings_13 (Variables|Default|GetWaterSettings))
  (bind _hud_reference_13 (Variables|Default|GetHUD%20Reference))
  (bind _initialcameratransform_12 (Variables|Default|GetInitialCameraTransform))
  (bind _asnew_game_instance (Utilities|Casting|CastToNewGameInstance (Game|GetGameInstance)))
  (if (== (Variables|/Game/PhysicalWaterSurface/Maps/DemoBlueprints/NewGameInstance.NewGameInstance_C|GetScale _asnew_game_instance) 0)
    ;[1 1 1] 0
    (bind _output_get (Variables|/Game/PhysicalWaterSurface/Blueprints/WaterSettings.WaterSettings_C|SetWindSpeed _watersettings_2 "NewEnumerator0"))
    (Variables|/Game/PhysicalWaterSurface/Blueprints/UI/SceneInfo.SceneInfo_C|SetWindSpeed _hud_reference (Utilities|String|EnumtoString _output_get))
    (bind _output_get_2 (Variables|/Game/PhysicalWaterSurface/Blueprints/WaterSettings.WaterSettings_C|SetFetchLength _watersettings_2 "NewEnumerator0"))
    (Variables|/Game/PhysicalWaterSurface/Blueprints/UI/SceneInfo.SceneInfo_C|SetFetchLength _hud_reference (Utilities|String|EnumtoString _output_get_2))
    (Default|UpdateHUD _hud_reference)
    (Default|ConstructionEvent _watersettings_2)
    (Utilities|FlowControl|Delay (Variables|Default|GetSceneDelay))
    (elif (== (Variables|/Game/PhysicalWaterSurface/Maps/DemoBlueprints/NewGameInstance.NewGameInstance_C|GetScale _asnew_game_instance) 1)
      ;[1 1 1] 1
      (bind _output_get_3 (Variables|/Game/PhysicalWaterSurface/Blueprints/WaterSettings.WaterSettings_C|SetWindSpeed _watersettings "NewEnumerator10"))
      (Variables|/Game/PhysicalWaterSurface/Blueprints/UI/SceneInfo.SceneInfo_C|SetWindSpeed _hud_reference_6 (Utilities|String|EnumtoString _output_get_3))
      (bind _output_get_4 (Variables|/Game/PhysicalWaterSurface/Blueprints/WaterSettings.WaterSettings_C|SetFetchLength _watersettings "NewEnumerator0"))
      (Variables|/Game/PhysicalWaterSurface/Blueprints/UI/SceneInfo.SceneInfo_C|SetFetchLength _hud_reference_6 (Utilities|String|EnumtoString _output_get_4))
      (Default|UpdateHUD _hud_reference_6)
      (Default|ConstructionEvent _watersettings)
      (Transformation|SetActorTransform (Variables|Default|GetCaneraActor) (Math|Transform|MakeTransform (+ (.location _initialcameratransform_5) "20.000000,10.000000,15.000000") (Math|Rotator|CombineRotators (.rotation _initialcameratransform_5) "0, 0, 0") "0, 0, 0"))
      (Utilities|FlowControl|Delay (Variables|Default|GetSceneDelay))
      (elif (== (Variables|/Game/PhysicalWaterSurface/Maps/DemoBlueprints/NewGameInstance.NewGameInstance_C|GetScale _asnew_game_instance) 2)
        ;[1 1 1] 2
        (bind _output_get_5 (Variables|/Game/PhysicalWaterSurface/Blueprints/WaterSettings.WaterSettings_C|SetWindSpeed _watersettings_3 "NewEnumerator1"))
        (Variables|/Game/PhysicalWaterSurface/Blueprints/UI/SceneInfo.SceneInfo_C|SetWindSpeed _hud_reference_3 (Utilities|String|EnumtoString _output_get_5))
        (bind _output_get_6 (Variables|/Game/PhysicalWaterSurface/Blueprints/WaterSettings.WaterSettings_C|SetFetchLength _watersettings_3 "NewEnumerator0"))
        (Variables|/Game/PhysicalWaterSurface/Blueprints/UI/SceneInfo.SceneInfo_C|SetFetchLength _hud_reference_3 (Utilities|String|EnumtoString _output_get_6))
        (Default|UpdateHUD _hud_reference_3)
        (Default|ConstructionEvent _watersettings_3)
        (Transformation|SetActorTransform (Variables|Default|GetCaneraActor) (Math|Transform|MakeTransform (+ (.location _initialcameratransform_2) "60.000000,30.000000,90.000000") (Math|Rotator|CombineRotators (.rotation _initialcameratransform_2) "0, 0, 0") "0, 0, 0"))
        (Utilities|FlowControl|Delay (* (Variables|Default|GetSceneDelay) 1.5))
        (elif (== (Variables|/Game/PhysicalWaterSurface/Maps/DemoBlueprints/NewGameInstance.NewGameInstance_C|GetScale _asnew_game_instance) 3)
          ;[1 1 1] 3
          (bind _output_get_7 (Variables|/Game/PhysicalWaterSurface/Blueprints/WaterSettings.WaterSettings_C|SetWindSpeed _watersettings_4 "NewEnumerator11"))
          (Variables|/Game/PhysicalWaterSurface/Blueprints/UI/SceneInfo.SceneInfo_C|SetWindSpeed _hud_reference_4 (Utilities|String|EnumtoString _output_get_7))
          (bind _output_get_8 (Variables|/Game/PhysicalWaterSurface/Blueprints/WaterSettings.WaterSettings_C|SetFetchLength _watersettings_4 "NewEnumerator0"))
          (Variables|/Game/PhysicalWaterSurface/Blueprints/UI/SceneInfo.SceneInfo_C|SetFetchLength _hud_reference_4 (Utilities|String|EnumtoString _output_get_8))
          (Default|UpdateHUD _hud_reference_4)
          (Default|ConstructionEvent _watersettings_4)
          (Transformation|SetActorTransform (Variables|Default|GetCaneraActor) (Math|Transform|MakeTransform (+ (.location _initialcameratransform_3) "300.000000,150.000000,250.000000") (Math|Rotator|CombineRotators (.rotation _initialcameratransform_3) "0, 0, 0") "0, 0, 0"))
          (Utilities|FlowControl|Delay (Variables|Default|GetSceneDelay))
          (elif (== (Variables|/Game/PhysicalWaterSurface/Maps/DemoBlueprints/NewGameInstance.NewGameInstance_C|GetScale _asnew_game_instance) 4)
            ;[1 1 1] 4
            (bind _output_get_9 (Variables|/Game/PhysicalWaterSurface/Blueprints/WaterSettings.WaterSettings_C|SetWindSpeed _watersettings_5 "NewEnumerator2"))
            (Variables|/Game/PhysicalWaterSurface/Blueprints/UI/SceneInfo.SceneInfo_C|SetWindSpeed _hud_reference_5 (Utilities|String|EnumtoString _output_get_9))
            (bind _output_get_10 (Variables|/Game/PhysicalWaterSurface/Blueprints/WaterSettings.WaterSettings_C|SetFetchLength _watersettings_5 "NewEnumerator0"))
            (Variables|/Game/PhysicalWaterSurface/Blueprints/UI/SceneInfo.SceneInfo_C|SetFetchLength _hud_reference_5 (Utilities|String|EnumtoString _output_get_10))
            (Default|UpdateHUD _hud_reference_5)
            (Default|ConstructionEvent _watersettings_5)
            (Transformation|SetActorTransform (Variables|Default|GetCaneraActor) (Math|Transform|MakeTransform (+ (.location _initialcameratransform_4) "1300.000000,500.000000,800.000000") (Math|Rotator|CombineRotators (.rotation _initialcameratransform_4) "0, 0, 0") "0, 0, 0"))
            (Utilities|FlowControl|Delay (* (Variables|Default|GetSceneDelay) 2.0))
            (elif (== (Variables|/Game/PhysicalWaterSurface/Maps/DemoBlueprints/NewGameInstance.NewGameInstance_C|GetScale _asnew_game_instance) 5)
              ;[1 1 1] 5
              (bind _output_get_11 (Variables|/Game/PhysicalWaterSurface/Blueprints/WaterSettings.WaterSettings_C|SetWindSpeed _watersettings_6 "NewEnumerator12"))
              (Variables|/Game/PhysicalWaterSurface/Blueprints/UI/SceneInfo.SceneInfo_C|SetWindSpeed _hud_reference_7 (Utilities|String|EnumtoString _output_get_11))
              (bind _output_get_12 (Variables|/Game/PhysicalWaterSurface/Blueprints/WaterSettings.WaterSettings_C|SetFetchLength _watersettings_6 "NewEnumerator1"))
              (Variables|/Game/PhysicalWaterSurface/Blueprints/UI/SceneInfo.SceneInfo_C|SetFetchLength _hud_reference_7 (Utilities|String|EnumtoString _output_get_12))
              (Default|UpdateHUD _hud_reference_7)
              (Default|ConstructionEvent _watersettings_6)
              (Transformation|SetActorTransform (Variables|Default|GetCaneraActor) (Math|Transform|MakeTransform (+ (.location _initialcameratransform_6) "800.000000,300.000000,800.000000") (Math|Rotator|CombineRotators (.rotation _initialcameratransform_6) "0, 0, 0") "0, 0, 0"))
              (Utilities|FlowControl|Delay (* (Variables|Default|GetSceneDelay) 1.5))
              (elif (== (Variables|/Game/PhysicalWaterSurface/Maps/DemoBlueprints/NewGameInstance.NewGameInstance_C|GetScale _asnew_game_instance) 6)
                ;[1 1 1] 6
                (bind _output_get_13 (Variables|/Game/PhysicalWaterSurface/Blueprints/WaterSettings.WaterSettings_C|SetWindSpeed _watersettings_7 "NewEnumerator3"))
                (Variables|/Game/PhysicalWaterSurface/Blueprints/UI/SceneInfo.SceneInfo_C|SetWindSpeed _hud_reference_13 (Utilities|String|EnumtoString _output_get_13))
                (bind _output_get_14 (Variables|/Game/PhysicalWaterSurface/Blueprints/WaterSettings.WaterSettings_C|SetFetchLength _watersettings_7 "NewEnumerator1"))
                (Variables|/Game/PhysicalWaterSurface/Blueprints/UI/SceneInfo.SceneInfo_C|SetFetchLength _hud_reference_13 (Utilities|String|EnumtoString _output_get_14))
                (Default|UpdateHUD _hud_reference_13)
                (Default|ConstructionEvent _watersettings_7)
                (Transformation|SetActorTransform (Variables|Default|GetCaneraActor) (Math|Transform|MakeTransform (+ (.location _initialcameratransform_12) "800.000000,200.000000,1200.000000") (Math|Rotator|CombineRotators (.rotation _initialcameratransform_12) "0, 0, 0") "0, 0, 0"))
                (Utilities|FlowControl|Delay (* (Variables|Default|GetSceneDelay) 1.5))
                (elif (== (Variables|/Game/PhysicalWaterSurface/Maps/DemoBlueprints/NewGameInstance.NewGameInstance_C|GetScale _asnew_game_instance) 7)
                  ;[1 1 1] 7
                  (bind _output_get_15 (Variables|/Game/PhysicalWaterSurface/Blueprints/WaterSettings.WaterSettings_C|SetWindSpeed _watersettings_9 "NewEnumerator4"))
                  (Variables|/Game/PhysicalWaterSurface/Blueprints/UI/SceneInfo.SceneInfo_C|SetWindSpeed _hud_reference_8 (Utilities|String|EnumtoString _output_get_15))
                  (bind _output_get_16 (Variables|/Game/PhysicalWaterSurface/Blueprints/WaterSettings.WaterSettings_C|SetFetchLength _watersettings_9 "NewEnumerator2"))
                  (Variables|/Game/PhysicalWaterSurface/Blueprints/UI/SceneInfo.SceneInfo_C|SetFetchLength _hud_reference_8 (Utilities|String|EnumtoString _output_get_16))
                  (Default|UpdateHUD _hud_reference_8)
                  (Default|ConstructionEvent _watersettings_9)
                  (Transformation|SetActorTransform (Variables|Default|GetCaneraActor) (Math|Transform|MakeTransform (+ (.location _initialcameratransform_7) "1000.000000,300.000000,800.000000") (Math|Rotator|CombineRotators (.rotation _initialcameratransform_7) "0, 0, 0") "0, 0, 0"))
                  (Utilities|FlowControl|Delay (* (Variables|Default|GetSceneDelay) 1.5))
                  (elif (== (Variables|/Game/PhysicalWaterSurface/Maps/DemoBlueprints/NewGameInstance.NewGameInstance_C|GetScale _asnew_game_instance) 8)
                    ;[1 1 1] 8
                    (bind _output_get_17 (Variables|/Game/PhysicalWaterSurface/Blueprints/WaterSettings.WaterSettings_C|SetWindSpeed _watersettings_10 "NewEnumerator5"))
                    (Variables|/Game/PhysicalWaterSurface/Blueprints/UI/SceneInfo.SceneInfo_C|SetWindSpeed _hud_reference_9 (Utilities|String|EnumtoString _output_get_17))
                    (bind _output_get_18 (Variables|/Game/PhysicalWaterSurface/Blueprints/WaterSettings.WaterSettings_C|SetFetchLength _watersettings_10 "NewEnumerator2"))
                    (Variables|/Game/PhysicalWaterSurface/Blueprints/UI/SceneInfo.SceneInfo_C|SetFetchLength _hud_reference_9 (Utilities|String|EnumtoString _output_get_18))
                    (Default|UpdateHUD _hud_reference_9)
                    (Default|ConstructionEvent _watersettings_10)
                    (Transformation|SetActorTransform (Variables|Default|GetCaneraActor) (Math|Transform|MakeTransform (+ (.location _initialcameratransform_8) "1000.000000,300.000000,800.000000") (Math|Rotator|CombineRotators (.rotation _initialcameratransform_8) "0, 0, 0") "0, 0, 0"))
                    (Utilities|FlowControl|Delay (* (Variables|Default|GetSceneDelay) 1.5))
                    (elif (== (Variables|/Game/PhysicalWaterSurface/Maps/DemoBlueprints/NewGameInstance.NewGameInstance_C|GetScale _asnew_game_instance) 9)
                      ;[1 1 1] 9
                      (bind _output_get_19 (Variables|/Game/PhysicalWaterSurface/Blueprints/WaterSettings.WaterSettings_C|SetWindSpeed _watersettings_11 "NewEnumerator6"))
                      (Variables|/Game/PhysicalWaterSurface/Blueprints/UI/SceneInfo.SceneInfo_C|SetWindSpeed _hud_reference_10 (Utilities|String|EnumtoString _output_get_19))
                      (bind _output_get_20 (Variables|/Game/PhysicalWaterSurface/Blueprints/WaterSettings.WaterSettings_C|SetFetchLength _watersettings_11 "NewEnumerator3"))
                      (Variables|/Game/PhysicalWaterSurface/Blueprints/UI/SceneInfo.SceneInfo_C|SetFetchLength _hud_reference_10 (Utilities|String|EnumtoString _output_get_20))
                      (Default|UpdateHUD _hud_reference_10)
                      (Default|ConstructionEvent _watersettings_11)
                      (Transformation|SetActorTransform (Variables|Default|GetCaneraActor) (Math|Transform|MakeTransform (+ (.location _initialcameratransform_9) "1000.000000,300.000000,800.000000") (Math|Rotator|CombineRotators (.rotation _initialcameratransform_9) "0, 0, 0") "0, 0, 0"))
                      (Utilities|FlowControl|Delay (* (Variables|Default|GetSceneDelay) 1.5))
                      (elif (== (Variables|/Game/PhysicalWaterSurface/Maps/DemoBlueprints/NewGameInstance.NewGameInstance_C|GetScale _asnew_game_instance) 10)
                        ;[1 1 1] 10
                        (bind _output_get_21 (Variables|/Game/PhysicalWaterSurface/Blueprints/WaterSettings.WaterSettings_C|SetWindSpeed _watersettings_12 "NewEnumerator7"))
                        (Variables|/Game/PhysicalWaterSurface/Blueprints/UI/SceneInfo.SceneInfo_C|SetWindSpeed _hud_reference_11 (Utilities|String|EnumtoString _output_get_21))
                        (bind _output_get_22 (Variables|/Game/PhysicalWaterSurface/Blueprints/WaterSettings.WaterSettings_C|SetFetchLength _watersettings_12 "NewEnumerator4"))
                        (Variables|/Game/PhysicalWaterSurface/Blueprints/UI/SceneInfo.SceneInfo_C|SetFetchLength _hud_reference_11 (Utilities|String|EnumtoString _output_get_22))
                        (Default|UpdateHUD _hud_reference_11)
                        (Default|ConstructionEvent _watersettings_12)
                        (Transformation|SetActorTransform (Variables|Default|GetCaneraActor) (Math|Transform|MakeTransform (+ (.location _initialcameratransform_10) "1000.000000,300.000000,800.000000") (Math|Rotator|CombineRotators (.rotation _initialcameratransform_10) "0, 0, 0") "0, 0, 0"))
                        (Utilities|FlowControl|Delay (* (Variables|Default|GetSceneDelay) 1.5))
                        (elif (== (Variables|/Game/PhysicalWaterSurface/Maps/DemoBlueprints/NewGameInstance.NewGameInstance_C|GetScale _asnew_game_instance) 11)
                          ;[1 1 1] 11
                          (bind _output_get_23 (Variables|/Game/PhysicalWaterSurface/Blueprints/WaterSettings.WaterSettings_C|SetWindSpeed _watersettings_13 "NewEnumerator8"))
                          (Variables|/Game/PhysicalWaterSurface/Blueprints/UI/SceneInfo.SceneInfo_C|SetWindSpeed _hud_reference_12 (Utilities|String|EnumtoString _output_get_23))
                          (bind _output_get_24 (Variables|/Game/PhysicalWaterSurface/Blueprints/WaterSettings.WaterSettings_C|SetFetchLength _watersettings_13 "NewEnumerator5"))
                          (Variables|/Game/PhysicalWaterSurface/Blueprints/UI/SceneInfo.SceneInfo_C|SetFetchLength _hud_reference_12 (Utilities|String|EnumtoString _output_get_24))
                          (Default|UpdateHUD _hud_reference_12)
                          (Default|ConstructionEvent _watersettings_13)
                          (Transformation|SetActorTransform (Variables|Default|GetCaneraActor) (Math|Transform|MakeTransform (+ (.location _initialcameratransform_11) "1000.000000,300.000000,800.000000") (Math|Rotator|CombineRotators (.rotation _initialcameratransform_11) "0, 0, 0") "0, 0, 0"))
                          (Utilities|FlowControl|Delay (* (Variables|Default|GetSceneDelay) 1.5))
                          (elif (== (Variables|/Game/PhysicalWaterSurface/Maps/DemoBlueprints/NewGameInstance.NewGameInstance_C|GetScale _asnew_game_instance) 12)
                            ;[1 1 1] 12
                            (bind _output_get_25 (Variables|/Game/PhysicalWaterSurface/Blueprints/WaterSettings.WaterSettings_C|SetWindSpeed _watersettings_8 "NewEnumerator9"))
                            (Variables|/Game/PhysicalWaterSurface/Blueprints/UI/SceneInfo.SceneInfo_C|SetWindSpeed _hud_reference_2 (Utilities|String|EnumtoString _output_get_25))
                            (bind _output_get_26 (Variables|/Game/PhysicalWaterSurface/Blueprints/WaterSettings.WaterSettings_C|SetFetchLength _watersettings_8 "NewEnumerator6"))
                            (Variables|/Game/PhysicalWaterSurface/Blueprints/UI/SceneInfo.SceneInfo_C|SetFetchLength _hud_reference_2 (Utilities|String|EnumtoString _output_get_26))
                            (Default|UpdateHUD _hud_reference_2)
                            (Default|ConstructionEvent _watersettings_8)
                            (Transformation|SetActorTransform (Variables|Default|GetCaneraActor) (Math|Transform|MakeTransform (+ (.location _initialcameratransform) "2000.000000,1000.000000,2000.000000") (Math|Rotator|CombineRotators (.rotation _initialcameratransform) "0, 0, 0") "0, 0, 0"))
                            (Utilities|FlowControl|Delay (* (Variables|Default|GetSceneDelay) 1.5))))))))))))))))

(fn ConstructionScript)